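; Game manager Blueprint that drives the overall game flow between Running, Win, Lose and Abandon states.
; Init creates the health HUD and end-screen widgets, initializes the player, then enters Running.
; SetState hides UI on each change, then shows the matching screen and toggles the mouse cursor.
; ResetGame teleports the player to the first PlayerStart and restores health; ShowHUD sets the health widget visible in both branches.
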(fn ConstructionScript)

(fn Init
  (CallFunction|CreateUI)
  (Default|Init (Variables|Default|GetMy%20Player))
  (CallFunction|SetState "NewEnumerator0"))

(fn SetState
  (params (New%20States :type MyGameStates%20Enum :default "NewEnumerator0"))
  (if (Utilities|Enum|NotEqual(Enum) New%20States (Variables|Default|GetCurrent%20Game%20State))
    (CallFunction|HideUI)
    (bind _output_get (Variables|Default|SetCurrent%20Game%20State New%20States))
    (switch Utilities|FlowControl|Switch|SwitchonMyGameStates _output_get
      (:NewEnumerator0
        (CallFunction|ShowMouse false)
        (CallFunction|ShowHUD true))
      (:NewEnumerator1
        (Widget|SetVisibility (Variables|Default|GetWidget%20Win) "Visible")
        (CallFunction|ShowMouse true :!label _label))
      (:NewEnumerator2
        (Widget|SetVisibility (Variables|Default|GetWidget%20Lose) "Visible")
        (goto _label))
      (:NewEnumerator3
        (Widget|SetVisibility (Variables|Default|GetWidget%20Abandon) "Visible")
        (goto _label)))))

(fn GetState
  (return (Variables|Default|GetCurrent%20Game%20State)))

(fn CreateUI
  (bind _returnvalue (UserInterface|CreateWidget "/Game/__MyContent/UI/Widget_Abandon.Widget_Abandon_C"))
  (bind _output_get (Variables|Default|SetWidget%20Abandon _returnvalue))
  (UserInterface|Viewport|AddtoViewport _output_get 0)
  (bind _returnvalue_2 (UserInterface|CreateWidget "/Game/__MyContent/UI/Widget_Win.Widget_Win_C"))
  (bind _output_get_2 (Variables|Default|SetWidget%20Win _returnvalue_2))
  (UserInterface|Viewport|AddtoViewport _output_get_2 0)
  (bind _returnvalue_3 (UserInterface|CreateWidget "/Game/__MyContent/UI/Lose_Widget.Lose_Widget_C"))
  (bind _output_get_3 (Variables|Default|SetWidget%20Lose _returnvalue_3))
  (UserInterface|Viewport|AddtoViewport _output_get_3 0)
  (bind _returnvalue_4 (UserInterface|CreateWidget "/Game/__MyContent/UI/Health_Widget.Health_Widget_C"))
  (bind _output_get_4 (Variables|Default|SetHealth _returnvalue_4))
  (UserInterface|Viewport|AddtoViewport _output_get_4 0))

(fn ResetGame
  (bind _my_player (Variables|Default|GetMy%20Player))
  (bind _outactors (Actor|GetAllActorsOfClass "/Script/Engine.PlayerStart"))
  (Transformation|SetActorLocation _my_player (Transformation|GetActorLocation (Utilities|Array|Get(acopy) _outactors)) false false)
  (Default|SetHealth _my_player 1e+02))

(fn ShowHUD
  (params (Visible :type Boolean))
  (bind _health (Variables|Default|GetHealth))
  (if Visible
    (Widget|SetVisibility _health "Visible")
    (else
      (Widget|SetVisibility _health "Visible"))))